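; Ladder (Escada) actor that detects when the first player character is level with it along the world X axis.
; Each tick it stores the X offset to the player and sets an Onlader flag when that offset is within a narrow range, ignoring Y and Z.
; Both branches enable player input on the actor, and debug prints show the offset and state; no climbing movement is implemented here.
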(event `self.ReceiveTick`
  (params (DeltaSeconds :type "Float (single-precision)"))
  (bind _returnvalue_x (`KismetMathLibrary.BreakVector` (`self.K2_GetActorLocation`)))
  (bind _returnvalue (`GameplayStatics.GetPlayerController` 0))
  (bind _returnvalue_x_2 (`KismetMathLibrary.BreakVector` (`self.K2_GetActorLocation` (`GameplayStatics.GetPlayerCharacter` 0))))
  (`|ExecutionSequence`
    (:`then_0`
      (set `self.dislader` (- _returnvalue_x _returnvalue_x_2)))
    (:`then_1`
      (`KismetSystemLibrary.PrintString` (`KismetStringLibrary.Conv_DoubleToString` (`self.dislader`))))
    (:`then_2`
      (if (`KismetMathLibrary.InRange_FloatFloat` (`self.dislader`) -10.0 10.0)
        (set `self.onlader` true)
        (`self.EnableInput` _returnvalue)
        (`KismetSystemLibrary.PrintString` "on")
        (else
          (set `self.onlader` false)
          (`self.EnableInput` _returnvalue)
          (`KismetSystemLibrary.PrintString` "off"))))))

(fn `UserConstructionScript`)