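; Paper2D actor "barra" that moves back and forth between two points, PontoA and PontoB, with an InterpToMovement component.
; The construction script turns both points into relative control points for that movement.
; On each reverse, a FlipFlop toggles the flipbook's X scale sign to mirror the sprite.
; An ActorLocation function resets Y to zero while keeping X and Z; Morte is an empty stub.
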(event `self.InterpToMovement.OnInterpToReverse`
  (params (ImpactResult :type "HitResult Structure (by ref)") (Time :type "Float (single-precision)"))
  (bind _paperflipbook (`self.PaperFlipbook`))
  (`/Engine/EditorBlueprintResources/StandardMacros.FlipFlop`
    (:`A`
      (`SceneComponent.SetWorldScale3D` _paperflipbook (0.5 0.5 0.5)))
    (:`B`
      (`SceneComponent.SetWorldScale3D` _paperflipbook (-0.5 0.5 0.5)))))

(fn `actor location`
  (bind (_returnvalue_x _returnvalue_y _returnvalue_z) (`KismetMathLibrary.BreakVector` (`self.K2_GetActorLocation`)))
  (`self.K2_SetActorLocation` (`KismetMathLibrary.MakeVector` _returnvalue_x 0.0 _returnvalue_z)))

(fn `morte`)

(fn `UserConstructionScript`
  (set `InterpToMovementComponent.ControlPoints` (`|MakeArray` (make `InterpControlPoint` (`self.PontoA`)) (make `InterpControlPoint` (`self.PontoB`))) (`self.InterpToMovement`)))