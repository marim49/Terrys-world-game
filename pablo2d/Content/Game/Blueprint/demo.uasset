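; Paper2D patrolling enemy that knocks back and lightly damages the Dude character on contact.
; InterpToMovement moves it between relative PontoA and PontoB points set in the construction script, mirroring the flipbook's X scale on each reversal via FlipFlop.
; Box overlap launches Dude using the sweep normal plus upward velocity, then applies damage.
; ActorLocation resets Y to zero, while Morte (death) is empty.
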(event `self.InterpToMovement.OnInterpToReverse`
  (params (ImpactResult :type "HitResult Structure (by ref)") (Time :type "Float (single-precision)"))
  (bind _paperflipbook (`self.PaperFlipbook`))
  (`/Engine/EditorBlueprintResources/StandardMacros.FlipFlop`
    (:`A`
      (`SceneComponent.SetWorldScale3D` _paperflipbook (0.1 0.1 0.1)))
    (:`B`
      (`SceneComponent.SetWorldScale3D` _paperflipbook (-0.1 0.1 0.1)))))

(event `self.Box.OnComponentBeginOverlap`
  (params (OverlappedComponent :type "PrimitiveComponent Object Reference") (OtherActor :type "Actor Object Reference") (OtherComp :type "PrimitiveComponent Object Reference") (OtherBodyIndex :type Integer) (bFromSweep :type Boolean) (SweepResult :type "HitResult Structure (by ref)"))
  (bind _asdude (cast `/Game/Game/Blueprint/Dude` OtherActor))
  (`Character.LaunchCharacter` _asdude (`KismetMathLibrary.MakeVector` (* (.x (`.Normal` (`GameplayStatics.BreakHitResult` SweepResult))) -500.0) 0.0 400.0) true true)
  (`GameplayStatics.ApplyDamage` _asdude 0.1 null null "/Script/Engine.DamageType"))

(fn `actor location`
  (bind (_returnvalue_x _returnvalue_y _returnvalue_z) (`KismetMathLibrary.BreakVector` (`self.K2_GetActorLocation`)))
  (`self.K2_SetActorLocation` (`KismetMathLibrary.MakeVector` _returnvalue_x 0.0 _returnvalue_z)))

(fn `morte`)

(fn `UserConstructionScript`
  (set `InterpToMovementComponent.ControlPoints` (`|MakeArray` (make `InterpControlPoint` (`self.PontoA`)) (make `InterpControlPoint` (`self.PontoB`))) (`self.InterpToMovement`)))