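; Climbable ladder ("escadas") that lets the Dude character climb while overlapping its Box.
; The construction script stacks collision-free Paper2D sprites, flattened in Z, at Runofset intervals over the height between Escadacomeco and Escadatop.
; It also derives the Box's Z scale and an added yaw from half that height, zeroing X and Y scale.
; Overlap begin sets the Dude's Bcanclimb flag; overlap end clears it and calls Endclimb.
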(event `self.Box.OnComponentBeginOverlap`
  (params (OverlappedComponent :type "PrimitiveComponent Object Reference") (OtherActor :type "Actor Object Reference") (OtherComp :type "PrimitiveComponent Object Reference") (OtherBodyIndex :type Integer) (bFromSweep :type Boolean) (SweepResult :type "HitResult Structure (by ref)"))
  (bind _asdude (cast `/Game/Game/Blueprint/Dude` OtherActor))
  (set `/Game/Game/Blueprint/Dude.bcanclimb` true _asdude))

(event `self.Box.OnComponentEndOverlap`
  (params (OverlappedComponent :type "PrimitiveComponent Object Reference") (OtherActor :type "Actor Object Reference") (OtherComp :type "PrimitiveComponent Object Reference") (OtherBodyIndex :type Integer))
  (bind _asdude (cast `/Game/Game/Blueprint/Dude` OtherActor))
  (set `/Game/Game/Blueprint/Dude.bcanclimb` false _asdude)
  (`/Game/Game/Blueprint/Dude.endclimb` _asdude))

(fn `UserConstructionScript`
  (bind _box (`self.Box`))
  (bind _runofset (`self.runofset`))
  (bind (_returnvalue_x _returnvalue_y _returnvalue_z) (`KismetMathLibrary.BreakVector` (- (`self.escadatop`) (`self.escadacomeco`))))
  (bind _returnvalue (/ _returnvalue_z 2.0))
  (for _index (range (+ (`KismetMathLibrary.FTrunc` (/ _returnvalue_z _runofset)) 1))
    (bind _returnvalue_2 (`AddComponent|NODE_AddPaperSpriteComponent-0` :`RelativeTransform` (`KismetMathLibrary.MakeTransform` (`KismetMathLibrary.MakeVector` 0.0 0.0 (* _index _runofset)) (struct) (1.0 1.0 0.1))))
    (`PaperSpriteComponent.SetSprite` _returnvalue_2 (`self.escadasprite`))
    (`PrimitiveComponent.SetCollisionEnabled` _returnvalue_2 "NoCollision"))
  (`SceneComponent.SetRelativeScale3D` _box (`KismetMathLibrary.MakeVector` 0.0 0.0 _returnvalue))
  (`SceneComponent.K2_AddRelativeRotation` _box (`KismetMathLibrary.MakeRotator` 0.0 0.0 _returnvalue) false false))