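; An actor that follows the first player's pawn every tick while that pawn is valid.
; It builds a start transform from the pawn's X and its own Y and Z, shifted by the Worldset offset, then interpolates that toward the pawn's transform with TInterpTo.
; After applying the result without sweep, it overrides the rotation with a fixed 90-degree turn, so the pawn's orientation is not followed.
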(event `self.ReceiveTick`
  (params (DeltaSeconds :type "Float (single-precision)"))
  (bind _returnvalue (`GameplayStatics.GetPlayerPawn` 0))
  (bind _returnvalue_2 (`self.GetTransform` _returnvalue))
  (`/Engine/EditorBlueprintResources/StandardMacros.IsValid` _returnvalue
    (:`Is Valid`
      (`self.K2_SetActorTransform` (`KismetMathLibrary.TInterpTo` (`KismetMathLibrary.MakeTransform` (+ (`KismetMathLibrary.MakeVector` (.x (.location _returnvalue_2)) (.y (.location (`self.GetTransform`))) (.z (.location (`self.GetTransform`)))) (`self.worldset`))) _returnvalue_2 DeltaSeconds))
      (`self.K2_SetActorRotation` (struct :`Yaw` -90.0)))))

(fn `UserConstructionScript`)